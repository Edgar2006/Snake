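; Test snake actor that builds a segmented body trailing a Head component, without using a spline.
; The construction script adds a row of static mesh segments spaced along negative X and stores them in an array.
; Each Tick chains them from the Head, with MoveBody interpolating every segment toward the previous one in relative space and rotating it to face that one.
; Unconnected leftover movement nodes, including a spline distance reset, never run.
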(event EventBeginPlay
  (Development|PrintString "Hello"))

(event EventTick
  (params (DeltaSeconds :type Float%20%28single-precision%29))
  (Variables|Default|SetParent (Variables|Default|GetHead))
  (for _array_element (Variables|Default|GetmeshArr)
    (bind _newtransform (CallFunction|MoveBody _array_element (Variables|Default|GetParent) DeltaSeconds))
    (Transformation|SetRelativeTransform _array_element _newtransform false false)
    (Variables|Default|SetParent _array_element)))

(fn ConstructionScript
  (for _index (range 0 (Variables|Default|GetCount))
    (bind _returnvalue (AddComponent|AddStaticMeshComponent false (Math|Transform|MakeTransform (Math|Vector|MakeVector (Math|Conversions|ToFloat(Integer) (* _index -50)) 0.0 0.0) "0, 0, 0" "1.000000,1.000000,1.000000")))
    (Components|StaticMesh|SetStaticMesh _returnvalue (Variables|Default|GetMesh))
    (Utilities|Array|Add (Variables|Default|GetmeshArr) _returnvalue)))

(fn MoveBody
  (params (Child :type Static%20Mesh%20Component%20Object%20Reference) (Parent :type Static%20Mesh%20Component%20Object%20Reference) (delataSecond :type Float%20%28double-precision%29))
  (bind _relativelocation (Variables|/Script/Engine.SceneComponent|GetRelativeLocation Child))
  (bind _interp_speed (Variables|Default|GetInterp%20Speed))
  (bind _relativelocation_2 (Variables|/Script/Engine.SceneComponent|GetRelativeLocation Parent))
  (bind _returnvalue (Math|Interpolation|VInterpTo _relativelocation _relativelocation_2 delataSecond _interp_speed))
  (return (Math|Transform|MakeTransform _returnvalue (Math|Rotator|FindLookatRotation _returnvalue (Variables|/Script/Engine.SceneComponent|GetRelativeLocation Parent)) "1.000000,1.000000,1.000000")))