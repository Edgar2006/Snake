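; Test snake body actor that lays a head mesh and a chain of body spline meshes back from the end of a spline.
; Construction spawns the collision-free segments; the Transform event places them by distance, either bending them with clamped tangents or positioning them rigidly, depending on WithTangent.
; Transform runs on construction and BeginPlay, not Tick; a two-second loop trims leading spline points while the spline exceeds the snake's length.
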(event Custom|Transform
  (for (_array_element _array_index) (Variables|Default|GetmeshArr)
    (if (Math|Conversions|ToBoolean(Integer) _array_index)
      (if (Variables|Default|GetwithTangent)
        (bind (_s_p _s_t _e_p _e_t) (CallFunction|GetSplineBodyTransform _array_index))
        (SplineMesh|SetStartandEnd _array_element _s_p _s_t _e_p _e_t true :!class /Script/Engine.SplineMeshComponent)
        (else
          (bind _returnvalue (CallFunction|GetSplineTransformWithoutTangent _array_index (Variables|Default|GetBodyLenght) "1.000000,1.000000,1.000000"))
          (Transformation|SetRelativeTransform _array_element _returnvalue false true)))
      (else
        (bind _returnvalue_2 (CallFunction|GetSplineTransformWithoutTangent _array_index (Variables|Default|GetOffset) "2.000000,1.000000,1.000000"))
        (Transformation|SetRelativeTransform _array_element _returnvalue_2 false true)))))

(event EventBeginPlay
  (CallFunction|Transform)
  (Utilities|FlowControl|Delay 2.0 :!label _label)
  (CallFunction|RemoveNoUsedPoints)
  (goto _label))

(event EventTick
  (params (DeltaSeconds :type Float%20%28single-precision%29)))

(fn ConstructionScript
  (for _index (range 0 (Variables|Default|GetCount))
    (bind _returnvalue (AddComponent|AddSplineMeshComponent false))
    (if (== _index 0)
      (Components|StaticMesh|SetStaticMesh _returnvalue (Variables|Default|GetHead))
      (else
        (Components|StaticMesh|SetStaticMesh _returnvalue (Variables|Default|GetBody))))
    (Collision|SetCollisionEnabled _returnvalue "NoCollision")
    (Utilities|Array|Add (Variables|Default|GetmeshArr) _returnvalue)
    (CallFunction|Transform)))

(fn GetSplineBodyTransform
  (params (Iterator :type Integer))
  (bind _returnvalue (- Iterator 1))
  (bind _offset (Variables|Default|GetOffset))
  (bind _offset_2 (Variables|Default|GetOffset))
  (bind _spline (Variables|Default|GetSpline))
  (bind _spline_2 (Variables|Default|GetSpline))
  (bind _spline_3 (Variables|Default|GetSpline))
  (bind _spline_4 (Variables|Default|GetSpline))
  (bind _returnvalue_2 (Spline|GetSplineLength _spline))
  (bind _returnvalue_3 (Spline|GetSplineLength _spline_2))
  (bind _returnvalue_4 (* _returnvalue _offset_2))
  (bind _returnvalue_5 (* Iterator _offset))
  (bind _returnvalue_6 (- _returnvalue_2 _returnvalue_4))
  (bind _returnvalue_7 (- _returnvalue_3 _returnvalue_5))
  (return (Spline|GetLocationatDistanceAlongSpline _spline_3 _returnvalue_7 "Local") (Math|Vector|ClampVectorSize (Spline|GetTangentatDistanceAlongSpline _spline_3 _returnvalue_7 "Local") 0.0 (Variables|Default|GetOffset)) (Spline|GetLocationatDistanceAlongSpline _spline_4 _returnvalue_6 "Local") (Math|Vector|ClampVectorSize (Spline|GetTangentatDistanceAlongSpline _spline_4 _returnvalue_6 "Local") 0.0 (Variables|Default|GetOffset))))

(fn GetSplineTransformWithoutTangent
  (params (Iterator :type Integer) (Offset :type Float%20%28double-precision%29) (Scale :type Vector))
  (bind _returnvalue (* Iterator Offset))
  (bind _spline (Variables|Default|GetSpline))
  (bind _spline_2 (Variables|Default|GetSpline))
  (bind _returnvalue_2 (Spline|GetSplineLength _spline))
  (bind _returnvalue_3 (- _returnvalue_2 _returnvalue))
  (bind _returnvalue_4 (Spline|GetTransformatDistanceAlongSpline _spline_2 _returnvalue_3 "Local" false))
  (bind (_location _rotation) (Math|Transform|BreakTransform _returnvalue_4))
  (return (Math|Transform|MakeTransform _location _rotation Scale)))

(fn RemoveNoUsedPoints
  (while (< (Spline|GetDistanceAlongSplineatSplinePoint (Variables|Default|GetSpline) 0) (- (Spline|GetSplineLength (Variables|Default|GetSpline)) (* (Variables|Default|GetCount) (Variables|Default|GetOffset))))
    (Spline|RemoveSplinePoint (Variables|Default|GetSpline) 0 true)))