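; Player character that spawns a BP_SnakeSpline on BeginPlay and feeds it path points and speed as the character moves.
; Tick sets the spline's Speed to the character's velocity magnitude divided by a variable.
; While IA_Move triggers, a boolean and short delay throttle a custom event that appends world-space spline points, offset along the mesh's right vector.
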(event Custom|CustomEvent
  (bind _mesh (Variables|Character|GetMesh))
  ;[1 1 1] Comment
  (Spline|AddSplinePoint (Variables|/Game/Player/test/BP_SnakeSpline.BP_SnakeSpline_C|GetSpline (Variables|Default|GetSpline)) (+ (Transformation|GetWorldLocation _mesh) (* (Math|Vector|GetRightVector _mesh) (Variables|Default|GetDistance))) "World" true)
  (Development|PrintString "Hello" true true "(R=0.000000,G=0.660000,B=1.000000,A=1.000000)" 1.0))

(event Input|EnhancedActionEvents|EnhancedInputActionIA_Move
  (params (ActionValue :type Vector%202D%20Structure) (ElapsedSeconds :type Float%20%28double-precision%29) (TriggeredSeconds :type Float%20%28double-precision%29) (InputAction :type Input%20Action%20Object%20Reference :default "/Game/Input/Action/IA_Move.IA_Move"))
  (:Triggered
    (if (Variables|Default|GetCondition)
      (CallFunction|CustomEvent)
      (Variables|Default|SetCondition false)
      (Utilities|FlowControl|Delay 3.0)
      (else
        (Utilities|FlowControl|Delay 0.2)
        (Variables|Default|SetCondition true)))))

(event EventBeginPlay
  ;[1 1 1] Comment
  (bind _returnvalue (Game|SpawnActorfromClass "/Game/Player/test/BP_SnakeSpline.BP_SnakeSpline_C" (Transformation|GetRelativeTransform (Variables|Default|GetCapsuleComponent)) "Undefined" "MultiplyWithRoot" 0 0))
  (Variables|Default|SetSpline _returnvalue))

(event EventTick
  (params (DeltaSeconds :type Float%20%28single-precision%29))
  (Variables|/Game/Player/test/BP_SnakeSpline.BP_SnakeSpline_C|SetSpeed (Variables|Default|GetSpline) (/ (Math|Vector|VectorLength (Transformation|GetVelocity)) (Variables|Default|GetNewVar))))

(fn ConstructionScript)