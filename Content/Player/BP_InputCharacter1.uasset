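; Player character that leads a spline-based snake, driven by Enhanced Input.
; On BeginPlay it attaches the head capsule to the mesh, spawns a BP_ASnakeSpline it owns and makes an initial move update.
; The IA_Move action repeats that update, passing the snake the mesh's forward vector and a position one unit ahead of the mesh.
; The character's own locomotion is not handled in this graph.
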(event Custom|CustomEvent
  (bind _mesh (Variables|Character|GetMesh))
  (bind _returnvalue (Math|Vector|GetForwardVector _mesh))
  ;[1 1 1] Comment
  (Class|ASnakeSpline|Move (Variables|Default|GetSnake) (+ (Transformation|GetWorldLocation _mesh) _returnvalue) _returnvalue))

(event Input|EnhancedActionEvents|EnhancedInputActionIA_Move
  (params (ActionValue :type Vector%202D%20Structure) (ElapsedSeconds :type Float%20%28double-precision%29) (TriggeredSeconds :type Float%20%28double-precision%29) (InputAction :type Input%20Action%20Object%20Reference :default "/Game/Input/Action/IA_Move.IA_Move"))
  ;[1 1 1] Comment
  (CallFunction|CustomEvent))

(event EventBeginPlay
  ;[1 1 1] Comment
  (Transformation|AttachComponentToComponent (Variables|Default|GetHeadCapsuleComponent) (Variables|Character|GetMesh) "None" "KeepRelative" "KeepRelative" "KeepRelative" true)
  (bind _returnvalue (Game|SpawnActorfromClass "/Game/Player/BP_ASnakeSpline.BP_ASnakeSpline_C" (Math|Transform|MakeTransform "0, 0, 0" "0, 0, 0" "1.000000,1.000000,1.000000") "Undefined" "MultiplyWithRoot" self 0))
  (Variables|Default|SetSnake _returnvalue)
  (CallFunction|CustomEvent))

(fn ConstructionScript)